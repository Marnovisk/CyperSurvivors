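; BP_AiSpawner is an actor that spawns a horde of melee enemies around its location.
; On BeginPlay it starts a looping timer and sets the horde size.
; Each tick of the timer spawns a BP_EnemyMeele at a random reachable navmesh point within a radius, until the count passes the limit.
; It prints the running count, then a limit-reached message while the timer keeps firing.
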(event Custom|Spawn%20Enemy
  (if (<= (Variables|Default|GetEnemyCount) (Variables|Default|GetHordeQtd))
    (Game|SpawnActorfromClass "/Game/Blueprints/Enemys/BP_EnemyMeele.BP_EnemyMeele_C" (Math|Transform|MakeTransform (.RandomLocation (AI|Navigation|GetRandomReachablePointinRadius (Transformation|GetActorLocation) 7e+02 0 0)) "0, 0, 0" "1.000000,1.000000,1.000000") "Undefined" "MultiplyWithRoot" 0 0)
    (bind _output_get (Variables|Default|SetEnemyCount (+ (Variables|Default|GetEnemyCount) 1)))
    (Development|PrintString (Utilities|String|ToString(Integer) _output_get))
    (else
      (Development|PrintString "Total de inimigos Atingidos"))))

(event EventBeginPlay
  (Utilities|Time|SetTimerbyEvent (delegate Custom|Spawn%20Enemy) 1.5 true)
  (Variables|Default|SetHordeQtd 10))

(fn ConstructionScript)