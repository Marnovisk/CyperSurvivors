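; BP_EnemyMeele is an enemy, named as a melee type, that handles its own health, death and XP reward.
; BeginPlay fills its health, and AnyDamage subtracts incoming damage until it runs out.
; On death it adds GivenXP to player 0's character, calls its XPWidget, destroys itself, prints the XP total and calls CheckEnemyDeath on the game mode.
; The graph contains no movement or attack logic.
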(event EventBeginPlay
  (bind _output_get (Variables|Default|SetVidaMax 1e+02))
  (Variables|Default|SetVidaAtual _output_get))

(event Collision|EventActorBeginOverlap
  (params (OtherActor :type Actor%20Object%20Reference))
  (|CallParentFunction OtherActor) ; This node is disabled and will not be called.\nDrag off pins to build functionality.
)

(event EventTick
  (params (DeltaSeconds :type Float%20%28single-precision%29))
  (|CallParentFunction DeltaSeconds) ; This node is disabled and will not be called.\nDrag off pins to build functionality.
)

(event Game|Damage|EventAnyDamage
  (params (Damage :type Float%20%28single-precision%29) (DamageType :type Damage%20Type%20Object%20Reference) (InstigatedBy :type Controller%20Object%20Reference) (DamageCauser :type Actor%20Object%20Reference))
  (Variables|Default|SetVidaAtual (- (Variables|Default|GetVidaAtual) Damage))
  (if (<= (Variables|Default|GetVidaAtual) 0.0)
    (bind _asbp_third_person_character (Utilities|Casting|CastToBP_ThirdPersonCharacter (Game|GetPlayerCharacter 0)))
    (bind _output_get (Variables|/Game/ThirdPerson/Blueprints/BP_ThirdPersonCharacter.BP_ThirdPersonCharacter_C|SetXP _asbp_third_person_character (+ (Variables|/Game/ThirdPerson/Blueprints/BP_ThirdPersonCharacter.BP_ThirdPersonCharacter_C|GetXP _asbp_third_person_character) (Variables|Default|GetGivenXP))))
    (Default|XPWidget _asbp_third_person_character)
    (Actor|DestroyActor)
    (Development|PrintString (Utilities|String|ToString(Float) _output_get))
    (bind _asbp_third_person_game_mode (Utilities|Casting|CastToBP_ThirdPersonGameMode (Game|GetGameMode)))
    (Default|CheckEnemyDeath _asbp_third_person_game_mode)))

(fn ConstructionScript
  (|CallParentFunction))