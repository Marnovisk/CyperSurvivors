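; Simple enemy Blueprint that takes damage and rewards the player with XP when killed.
; Health starts at a fixed maximum on BeginPlay, and AnyDamage subtracts incoming damage from it.
; At zero or below, it adds GivenXP to player 0's BP_ThirdPersonCharacter regardless of damage source, calls XPWidget, destroys itself and prints the XP total.
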(event EventBeginPlay
  (bind _output_get (Variables|Default|SetVidaMax 1e+02))
  (Variables|Default|SetVidaAtual _output_get))

(event Collision|EventActorBeginOverlap
  (params (OtherActor :type Actor%20Object%20Reference)))

(event EventTick
  (params (DeltaSeconds :type Float%20%28single-precision%29)))

(event Game|Damage|EventAnyDamage
  (params (Damage :type Float%20%28single-precision%29) (DamageType :type Damage%20Type%20Object%20Reference) (InstigatedBy :type Controller%20Object%20Reference) (DamageCauser :type Actor%20Object%20Reference))
  (Variables|Default|SetVidaAtual (- (Variables|Default|GetVidaAtual) Damage))
  (if (<= (Variables|Default|GetVidaAtual) 0.0)
    (bind _asbp_third_person_character (Utilities|Casting|CastToBP_ThirdPersonCharacter (Game|GetPlayerCharacter 0)))
    (bind _output_get (Variables|/Game/ThirdPerson/Blueprints/BP_ThirdPersonCharacter.BP_ThirdPersonCharacter_C|SetXP _asbp_third_person_character (+ (Variables|/Game/ThirdPerson/Blueprints/BP_ThirdPersonCharacter.BP_ThirdPersonCharacter_C|GetXP _asbp_third_person_character) (Variables|Default|GetGivenXP))))
    (Default|XPWidget _asbp_third_person_character)
    (Actor|DestroyActor)
    (Development|PrintString (Utilities|String|ToString(Float) _output_get))))

(fn ConstructionScript)